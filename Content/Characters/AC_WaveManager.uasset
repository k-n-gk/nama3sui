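; Wave manager actor that tracks enemy wave completion across all AC_EnemySpawn actors, which it gathers on BeginPlay.
; CompleteEachWave increments CompCnt until it equals the spawner count, then advances WaveCnt without resetting CompCnt.
; It calls BeginNextWave, empty here, while under five waves; afterwards it uses ApplyDamage as a signal to the Level Blueprint's damage event.
; The delayed first-wave start is disconnected and never runs.
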(event Custom|BeginNextWave)

(event Custom|CompleteEachWave
  (if (== (Utilities|Array|Length (Variables|Default|GetENSpawns)) (Variables|Default|GetCompCnt))
    (bind _result (Math|Integer|IncrementInt (Variables|Default|GetWaveCnt))
      (:%20%20
        (if (< _result 5)
          (CallFunction|BeginNextWave)
          (else
            (Game|Damage|ApplyDamage 0 1.0 0 0) ; LevelBPのDamageEventを呼べる
          ))))
    (else
      (Math|Integer|IncrementInt (Variables|Default|GetCompCnt)))))

(event EventBeginPlay
  (bind _outactors (Actor|GetAllActorsOfClass "/Game/Characters/AC_EnemySpawn.AC_EnemySpawn_C"))
  (Variables|Default|SetENSpawns _outactors))

(event EventActorBeginOverlap
  (params (OtherActor :type Actor%20Object%20Reference)))

(event EventTick
  (params (DeltaSeconds :type Float%20%28single-precision%29)))

(fn ConstructionScript)