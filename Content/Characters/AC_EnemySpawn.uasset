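; Enemy spawner that spawns two enemy types at its own location, wave by wave.
; Each timed SpawnEnemy call reads the current position's per-type counts and runs two ForLoopWithDelay macros with separate intervals, each inclusive from zero.
; DeltaEmitted flags join both branches before scheduling the next position via NextTime or calling ParentCompleteEachWave after the last.
; BeginPlay and BeginNextWave both start the timer.
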(event Custom|SpawnEnemy
  (bind _self self)
  (bind _enemyperwave (Variables|Default|GetEnemyPerWave))
  (bind _wavecnt (Variables|Default|GetWaveCnt))
  (bind _wavecnt_2 (Variables|Default|GetWaveCnt))
  (bind _deltaspawntime (Variables|Default|GetDeltaSpawnTime))
  (bind _enemyperwave_2 (Variables|Default|GetEnemyPerWave))
  (bind _item (Utilities|Array|Get(acopy) _enemyperwave _wavecnt))
  (bind _item_2 (Utilities|Array|Get(acopy) _enemyperwave_2 _wavecnt_2))
  (bind _returnvalue (Transformation|GetActorLocation _self))
  (bind _returnvalue_2 (Transformation|GetActorRotation _self))
  (bind (_nexttime _en_01 _en_02) (Utilities|Struct|BreakEnemyPerWave _item_2))
  (bind _nexttime_2 (Utilities|Struct|BreakEnemyPerWave _item))
  ;[1 1 1] SpawnEnemy
  (Utilities|FlowControl|Sequence
    (:then_0
      (if (!= (Utilities|Array|Get(acopy) _en_01 (Variables|Default|GetPositionInWave)) 0)
        (Utilities|ForLoopwithDelay 0 (Utilities|Array|Get(acopy) _en_01 (Variables|Default|GetPositionInWave)) (Utilities|Array|Get(acopy) _deltaspawntime)
          (:LoopBody
            (AI|SpawnAIFromClass "/Game/Characters/CH_Enemy_01.CH_Enemy_01_C" 0 _returnvalue _returnvalue_2 true))
          (:Completed
            (Utilities|Array|SetArrayElem (Variables|Default|GetDeltaEmitted) 0 true :!label _label)
            ;;[1 1 1] Pos in Wave進行及びWave進行
            (if (and (Utilities|Array|Get(acopy) (Variables|Default|GetDeltaEmitted)) (Utilities|Array|Get(acopy) (Variables|Default|GetDeltaEmitted) 1)) :!label _label_2
              (Variables|Default|SetDeltaEmitted (Utilities|Array|MakeArray false false))
              (if (< (Variables|Default|GetPositionInWave) (- (Utilities|Array|Length _nexttime_2) 1))
                (Utilities|Time|SetTimerbyFunctionName self "SpawnEnemy" (Utilities|Array|Get(acopy) _nexttime_2 (Variables|Default|GetPositionInWave)))
                (Math|Integer|IncrementInt (Variables|Default|GetPositionInWave))
                (else
                  (Variables|Default|SetPositionInWave 0)
                  (|CallParentFunction))))))
        (else
          (goto _label))))
    (:then_1
      (if (!= (Utilities|Array|Get(acopy) _en_02 (Variables|Default|GetPositionInWave)) 0)
        (Utilities|ForLoopwithDelay 0 (Utilities|Array|Get(acopy) _en_02 (Variables|Default|GetPositionInWave)) (Utilities|Array|Get(acopy) _deltaspawntime 1)
          (:LoopBody
            (AI|SpawnAIFromClass "/Game/Characters/CH_Enemy_02.CH_Enemy_02_C" 0 _returnvalue _returnvalue_2 true))
          (:Completed
            (Utilities|Array|SetArrayElem (Variables|Default|GetDeltaEmitted) 1 true :!label _label_3)
            (goto _label_2)))
        (else
          (goto _label_3))))))

(event EventBeginNextWave
  (Utilities|Time|SetTimerbyFunctionName self "SpawnEnemy" 0.1))

(event EventBeginPlay
  (Utilities|Time|SetTimerbyFunctionName self "SpawnEnemy" 0.1))

(fn ConstructionScript)