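; Projectile actor that homes in on the first player's pawn and has a limited lifetime.
; BeginPlay sets the pawn's root component as the ProjectileMovement homing target.
; On overlap with any actor, it applies a small fixed-magnitude acceleration force to its updated primitive, pointing away from that actor.
; Tick counts frames and destroys the projectile past a threshold, so its lifetime depends on frame rate.
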(event EventBeginPlay
  (Variables|/Script/Engine.ProjectileMovementComponent|SetHomingTargetComponent (Variables|Default|GetProjectileMovement) (VehicleSound|GetRootComponent (Game|Player|GetPlayerPawn 0))))

(event EventActorBeginOverlap
  (params (OtherActor :type Actor%20Object%20Reference))
  (bind _returnvalue (Transformation|GetActorLocation OtherActor))
  (bind _projectilemovement (Variables|Default|GetProjectileMovement))
  (bind _updatedprimitive (Variables|/Script/Engine.MovementComponent|GetUpdatedPrimitive _projectilemovement))
  (bind _returnvalue_2 (Transformation|GetWorldLocation _updatedprimitive))
  (bind _returnvalue_3 (- _returnvalue_2 _returnvalue))
  (if true
    (Physics|AddForce (Variables|/Script/Engine.MovementComponent|GetUpdatedPrimitive _projectilemovement) (* _returnvalue_3 (/ 1e+01 (Math|Vector|VectorLength _returnvalue_3))) "None" true)))

(event EventTick
  (params (DeltaSeconds :type Float%20%28single-precision%29))
  (bind _output_get (Variables|Default|Setcount (+ (Variables|Default|Getcount) 1)))
  (if (> _output_get 300)
    (Actor|DestroyActor)
    (Variables|Default|Setcount 0)))

(fn ConstructionScript)