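; Projectile-like actor with a physics Sphere that seeks a hardcoded world point while veering away from actors it overlaps.
; Each tick it applies force toward that point, resets velocity to a constant speed and rotates the StaticMesh to face travel.
; Overlaps beyond a minimum distance add a horizontal repulsion force, then run the same steering chain.
; A tick counter destroys the actor after a fixed frame count, so lifetime depends on frame rate.
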(event EventBeginPlay)

(event Collision|EventActorBeginOverlap
  (params (OtherActor :type Actor%20Object%20Reference))
  (bind _returnvalue (Transformation|GetActorLocation OtherActor))
  (bind _sphere (Variables|Default|GetSphere))
  (bind _sphere_2 (Variables|Default|GetSphere))
  (bind _returnvalue_2 (Transformation|GetWorldLocation _sphere))
  (bind _returnvalue_3 (- _returnvalue_2 _returnvalue))
  (bind _returnvalue_4 (Math|Vector|VectorLength _returnvalue_3))
  (if (> _returnvalue_4 2e+01)
    (Physics|AddForce _sphere (* (* _returnvalue_3 (/ 1e+01 _returnvalue_4)) "1.000000,1.000000,0.000000") "None" false)
    (Physics|AddForce _sphere_2 (* (Math|Vector|Normalize (- "-90.000000,5000.000000, 0" (Transformation|GetWorldLocation _sphere_2))) 2) "None" false)
    (bind _returnvalue_5 (Physics|GetPhysicsLinearVelocity _sphere_2 "None"))
    (Physics|SetPhysicsLinearVelocity _sphere_2 (* (Math|Vector|Normalize _returnvalue_5) 75.0) false "None")
    (Transformation|SetRelativeRotation (Variables|Default|GetStaticMesh) (Math|Conversions|RotationFromXVector (* (Math|Vector|Normalize _returnvalue_5) 75.0)) false false)))

(event EventTick
  (params (DeltaSeconds :type Float%20%28single-precision%29))
  (bind _sphere (Variables|Default|GetSphere))
  (bind _output_get (Variables|Default|Setcount (+ (Variables|Default|Getcount) 1)))
  (if (> _output_get 280)
    (Actor|DestroyActor)
    (Variables|Default|Setcount 0)
    (else
      (Physics|AddForce _sphere (* (Math|Vector|Normalize (- "-90.000000,5000.000000, 0" (Transformation|GetWorldLocation _sphere))) 2) "None" false)
      (bind _returnvalue (Physics|GetPhysicsLinearVelocity _sphere "None"))
      (Physics|SetPhysicsLinearVelocity _sphere (* (Math|Vector|Normalize _returnvalue) 75.0) false "None")
      (Transformation|SetRelativeRotation (Variables|Default|GetStaticMesh) (Math|Conversions|RotationFromXVector (* (Math|Vector|Normalize _returnvalue) 75.0)) false false))))

(fn ConstructionScript)