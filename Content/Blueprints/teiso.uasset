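; The teiso Blueprint is an actor that grows after it appears and removes itself on a signal from the nama3gamestate game state.
; Each Tick adds a fixed, frame-rate-dependent step to the root component's world scale, applied uniformly from its Y value, until X reaches a cap.
; Tick also polls the game state's Del flag, and when it is set the actor destroys itself and deducts a fixed amount from Cost.
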(event EventBeginPlay)

(event Collision|EventActorBeginOverlap
  (params (OtherActor :type Actor%20Object%20Reference)))

(event EventTick
  (params (DeltaSeconds :type Float%20%28single-precision%29))
  (bind _returnvalue (Game|GetGameState))
  (bind _defaultsceneroot (Variables|Default|GetDefaultSceneRoot))
  (bind _returnvalue_2 (Transformation|GetWorldScale _defaultsceneroot))
  (bind _asnama_3gamestate (Utilities|Casting|CastTonama3gamestate _returnvalue))
  (bind (_x _y) (Math|Vector|BreakVector _returnvalue_2))
  (bind _returnvalue_3 (+ _y 0.008))
  (if (> 0.8 _x)
    (Transformation|SetWorldScale3D _defaultsceneroot (Math|Vector|MakeVector _returnvalue_3 _returnvalue_3 _returnvalue_3)))
  (if (Variables|/Game/Blueprints/nama3gamestate.nama3gamestate_C|GetDel _asnama_3gamestate)
    (Actor|DestroyActor)
    (Variables|/Game/Blueprints/nama3gamestate.nama3gamestate_C|Setcost _asnama_3gamestate (- (Variables|/Game/Blueprints/nama3gamestate.nama3gamestate_C|Getcost _asnama_3gamestate) 3))))

(fn ConstructionScript)