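; Target point Blueprint that acts as a repeating spawner, creating Projec2 actors at its own transform.
; Tick increments a frame counter and spawns when it passes a threshold, then partially resets it, so the rate depends on frame rate.
; An uncalled helper function is meant to randomly return the owner cast to tatestone or hunastone, but RandomInteger(1) always yields zero, leaving the hunastone branch unreachable.
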(event EventBeginPlay)

(event EventActorBeginOverlap
  (params (OtherActor :type Actor%20Object%20Reference)))

(event EventTick
  (params (DeltaSeconds :type Float%20%28single-precision%29))
  (bind _output_get (Variables|Default|SetNewVar_0 (+ (Variables|Default|GetNewVar_0) 1)))
  (if (> _output_get 20)
    (Game|SpawnActorfromClass "/Game/Blueprints/projec2.projec2_C" (Transformation|GetActorTransform) "Undefined" 0 0)
    (Variables|Default|SetNewVar_0 5)))

(fn ConstructionScript)

(fn 新規関数0
  (bind _returnvalue (Math|Random|RandomInteger 1))
  (bind _returnvalue_2 (Components|GetOwner))
  (if (== _returnvalue 0)
    (bind _astatestone (Utilities|Casting|CastTotatestone _returnvalue_2))
    (Variables|Default|Setrandom _astatestone)
    (return (Variables|Default|Getrandom))
    (elif (== _returnvalue 1)
      (bind _ashunastone (Utilities|Casting|CastTohunastone _returnvalue_2))
      (Variables|Default|Setrandom _ashunastone)
      (return (Variables|Default|Getrandom)))))