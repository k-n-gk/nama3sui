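; Stone actor (yokostone) that grows into place and removes itself when the game state signals deletion.
; Each Tick raises its static mesh's uniform world scale by a fixed, frame-rate-dependent step, based on Z, until it reaches full size.
; Tick also polls the Del flag on nama3gamestate; when set, the actor destroys itself and decrements the shared Cost counter.
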(event EventBeginPlay)

(event EventActorBeginOverlap
  (params (OtherActor :type Actor%20Object%20Reference)))

(event EventTick
  (params (DeltaSeconds :type Float%20%28single-precision%29))
  (bind _returnvalue (Game|GetGameState))
  (bind _staticmeshcomponent (Variables|Debug|GetStaticMeshComponent))
  (bind _returnvalue_2 (Transformation|GetWorldScale _staticmeshcomponent))
  (bind _asnama_3gamestate (Utilities|Casting|CastTonama3gamestate _returnvalue))
  (bind _z (Math|Vector|BreakVector _returnvalue_2))
  (bind _returnvalue_3 (+ _z 0.01))
  (if (> 1.0 _z)
    (Transformation|SetWorldScale3D _staticmeshcomponent (Math|Vector|MakeVector _returnvalue_3 _returnvalue_3 _returnvalue_3)))
  (if (Variables|/Game/Blueprints/nama3gamestate.nama3gamestate_C|GetDel _asnama_3gamestate)
    (Actor|DestroyActor)
    (Variables|/Game/Blueprints/nama3gamestate.nama3gamestate_C|Setcost _asnama_3gamestate (- (Variables|/Game/Blueprints/nama3gamestate.nama3gamestate_C|Getcost _asnama_3gamestate) 1))))

(fn ConstructionScript)