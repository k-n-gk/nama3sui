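; yubicol is a cursor-following probe actor that flags on the game state whether it has touched a stone.
; Each tick it moves its root to the Visibility trace hit under the cursor, aligned to the surface normal.
; On begin overlap it loops the other actor's tags, setting ColOK false for "stone" and true otherwise, so the last tag wins.
; No end-overlap handler resets the flag.
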(event EventBeginPlay
  (Transformation|SetActorLocation "0, 0,60.000000" true false))

(event EventActorBeginOverlap
  (params (OtherActor :type Actor%20Object%20Reference))
  (bind _returnvalue (Game|GetGameState))
  (bind _asnama_3gamestate (Utilities|Casting|CastTonama3gamestate _returnvalue))
  (for _array_element (Variables|/Script/Engine.Actor|GetTags OtherActor)
    (if (Utilities|Name|Equal(Name) _array_element "stone")
      (Variables|/Game/Blueprints/nama3gamestate.nama3gamestate_C|SetcolOK _asnama_3gamestate false)
      (else
        (Variables|/Game/Blueprints/nama3gamestate.nama3gamestate_C|SetcolOK _asnama_3gamestate true)))))

(event EventTick
  (params (DeltaSeconds :type Float%20%28single-precision%29))
  (bind _returnvalue (Game|GetPlayerController 0))
  (bind _hitresult (Game|Player|GetHitResultUnderCursorbyChannel _returnvalue "TraceTypeQuery1" true))
  (bind (_bblockinghit _binitialoverlap _time _location _impactpoint _normal _impactnormal) (Collision|BreakHitResult _hitresult))
  (Transformation|SetWorldLocationAndRotation (Variables|Default|GetDefaultSceneRoot) _location (Math|Rotator|MakeRotationfromAxes _impactnormal "0, 0, 0" "0, 0, 0") false false))

(fn ConstructionScript)