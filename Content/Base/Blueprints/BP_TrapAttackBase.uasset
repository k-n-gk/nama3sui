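; Base trap actor with a garden lantern, pulsing ripple and fire attack against enemies, leaving Attack empty for child Blueprints.
; Tick shrinks the ripple plane and resets it at minimum scale, opening a frame-counted input window that ResetCount consumes, returning success.
; While EradiationTime remains, fire shows and a forward sphere trace damages enemies with effect and sound.
; The construction script applies ripple and lantern colors through dynamic materials.
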(event Custom|Attack
  ;[1 1 1] 継承先で攻撃の実装
)

(event EventTick
  (params (DeltaSeconds :type Float%20%28single-precision%29))
  (bind _eradiationtime (Variables|Default|GetEradiationTime))
  (bind _sm_plane (Variables|Default|GetSM_Plane))
  (bind _p_fire (Variables|Default|GetP_Fire))
  (bind _returnvalue (Transformation|GetWorldScale _sm_plane))
  (bind _returnvalue_2 (> _eradiationtime 0.1))
  (bind _returnvalue_3 (Transformation|GetWorldLocation _p_fire))
  ;[1 1 1] 波紋の拡縮
  (Utilities|FlowControl|Sequence
    (:then_0
      ;;[1 1 1] ボタン入力時間の減算
      (if (> (Variables|Default|GetPushCount) 0.0)
        (Math|Float|DecrementFloat (Variables|Default|GetPushCount))))
    (:then_1
      (if (<= (Math|Vector|VectorLength _returnvalue) (Variables|Default|GetMinScale))
        (Transformation|SetWorldScale3D _sm_plane (Math|Conversions|ToVector(Float) (Variables|Default|GetMaxScale)))
        (if (<= (Variables|Default|GetPushCount) 0.0)
          (Variables|Default|SetPushCount (Variables|Default|GetButtonTimeIn))
          (Effects|SpawnEmitteratLocation "/Game/Effects/Particles/P_PushEffect.P_PushEffect" (Transformation|GetActorLocation) (Transformation|GetActorRotation)))
        (else
          (Transformation|SetWorldScale3D _sm_plane (Math|Vector|Lerp(Vector) _returnvalue "0, 0, 0" (* DeltaSeconds (Variables|Default|GetScaleSpeed)))))))
    (:then_2
      ;[1 1 1] SphereCastで攻撃の当たり判定をとる
      (if _returnvalue_2
        (bind _outhit (Class|KismetSystemLibrary|SphereTraceSingleNEW _returnvalue_3 (+ _returnvalue_3 (* (Math|Vector|GetForwardVector _p_fire) (Variables|Default|GetCollisionDistance))) 5e+01 "TraceTypeQuery3" false 0 "ForOneFrame" true))
        (if (.bSuccess (Utilities|Casting|CastToCH_Enemy_Parent (.HitActor (Collision|BreakHitResult _outhit))))
          (Effects|SpawnEmitteratLocation "/Game/Effects/Particles/P_HitEffect.P_HitEffect" (.Location (Collision|BreakHitResult _outhit)) (Transformation|GetActorRotation (.HitActor (Collision|BreakHitResult _outhit))))
          (Game|Damage|ApplyDamage (.AsCH%20Enemy%20Parent (Utilities|Casting|CastToCH_Enemy_Parent (.HitActor (Collision|BreakHitResult _outhit)))) (Variables|Default|GetDamage) 0 0)
          (Audio|PlaySound2D 0))))
    (:then_3
      ;;[1 1 1] Comment攻撃エフェクトの描画判定
      (Math|Float|DecrementFloat _eradiationtime
        (:%20%20
          (Rendering|SetVisibility (Variables|Default|GetP_Fire) _returnvalue_2 false))))))

(fn ConstructionScript
  (bind _sm_plane (Variables|Default|GetSM_Plane))
  ;[1 1 1] 色と最大拡大値の反映
  (bind _returnvalue (Rendering|Material|CreateDynamicMaterialInstance _sm_plane 0 0 :!class /Script/Engine.PrimitiveComponent))
  (Rendering|Material|SetVectorParameterValue _returnvalue "BaseColor" (Variables|Default|GetWaveBaseColor) :!class /Script/Engine.MaterialInstanceDynamic)
  (Transformation|SetWorldScale3D _sm_plane (Math|Conversions|ToVector(Float) (Variables|Default|GetMaxScale)))
  (bind _returnvalue_2 (Rendering|Material|CreateDynamicMaterialInstance (Variables|Default|GetSM_GardenLantern) 0 0 :!class /Script/Engine.PrimitiveComponent))
  (Rendering|Material|SetVectorParameterValue _returnvalue_2 "BaseColor" (Variables|Default|GetGardenLanternColor) :!class /Script/Engine.MaterialInstanceDynamic)
  (|CallParentFunction))

(fn ResetCount
  ;[1 1 1] ボタン入力受付時間の初期化
  (if (> (Variables|Default|GetPushCount) 0.0)
    (Variables|Default|SetPushCount 0.0)
    (return true)
    (else
      (return false))))