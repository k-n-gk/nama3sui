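; CameraMover is a controller that pans and zooms the player's flying camera pawn.
; Both movement axes feed one AddMovementInput call, and Tick clamps the pawn's X and Y within a symmetric MoveRange around the world origin.
; Held zoom inputs run gated retriggerable-delay loops that step BP_FlyingCamera's spring arm length within limits.
; ZoomIn lengthens the arm and ZoomOut shortens it, opposite to their names.
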(event EventBeginPlay)

(event EventTick
  (params (DeltaSeconds :type Float%20%28single-precision%29))
  (bind _returnvalue (Pawn|GetControlledPawn))
  (bind _moverange (Variables|Default|GetMoveRange))
  (Transformation|SetActorLocation _returnvalue (Math|Vector|MakeVector (Math|Float|Clamp(Float) (.x (Transformation|GetActorLocation _returnvalue)) (* (.x _moverange) -1.0) (.x _moverange)) (Math|Float|Clamp(Float) (.y (Transformation|GetActorLocation _returnvalue)) (* (.y _moverange) -1.0) (.y _moverange)) (.z (Transformation|GetActorLocation (Pawn|GetControlledPawn)))) false false))

(event Input|ActionEvents|InputActionZoomOut
  (params (Key :type Key%20Structure :default "AnyKey"))
  (:Pressed
    (Utilities|FlowControl|Sequence
      (:then_0
        (goto _label Open))
      (:then_1
        (Utilities|FlowControl|Gate true :!label _label
          (:Exit
            (Utilities|FlowControl|Sequence
              (:then_0
                (bind _asbp_flying_camera (Utilities|Casting|CastToBP_FlyingCamera (Game|Player|GetPlayerPawn 0)))
                (if (not (<= (Variables|/Script/Engine.SpringArmComponent|GetTargetArmLength (Variables|/Game/GamePlay/Blueprints/BP_FlyingCamera.BP_FlyingCamera_C|GetSpringArm _asbp_flying_camera)) 0.0))
                  (Variables|/Script/Engine.SpringArmComponent|SetTargetArmLength (Variables|/Game/GamePlay/Blueprints/BP_FlyingCamera.BP_FlyingCamera_C|GetSpringArm _asbp_flying_camera) (- (Variables|/Script/Engine.SpringArmComponent|GetTargetArmLength (Variables|/Game/GamePlay/Blueprints/BP_FlyingCamera.BP_FlyingCamera_C|GetSpringArm _asbp_flying_camera)) 25.0))))
              (:then_1
                (Utilities|FlowControl|RetriggerableDelay 0.01)
                (goto _label))))))))
  (:Released
    (goto _label Close)))

(event Input|ActionEvents|InputActionZoomIn
  (params (Key :type Key%20Structure :default "AnyKey"))
  (:Pressed
    (Utilities|FlowControl|Sequence
      (:then_0
        (goto _label Open))
      (:then_1
        (Utilities|FlowControl|Gate true :!label _label
          (:Exit
            (Utilities|FlowControl|Sequence
              (:then_0
                (bind _asbp_flying_camera (Utilities|Casting|CastToBP_FlyingCamera (Game|Player|GetPlayerPawn 0)))
                (if (not (>= (Variables|/Script/Engine.SpringArmComponent|GetTargetArmLength (Variables|/Game/GamePlay/Blueprints/BP_FlyingCamera.BP_FlyingCamera_C|GetSpringArm _asbp_flying_camera)) 4e+03))
                  (Variables|/Script/Engine.SpringArmComponent|SetTargetArmLength (Variables|/Game/GamePlay/Blueprints/BP_FlyingCamera.BP_FlyingCamera_C|GetSpringArm _asbp_flying_camera) (+ (Variables|/Script/Engine.SpringArmComponent|GetTargetArmLength (Variables|/Game/GamePlay/Blueprints/BP_FlyingCamera.BP_FlyingCamera_C|GetSpringArm _asbp_flying_camera)) 25.0))))
              (:then_1
                (Utilities|FlowControl|RetriggerableDelay 0.01)
                (goto _label))))))))
  (:Released
    (goto _label Close)))

(event Input|AxisEvents|InputAxisMoveRight
  (params (AxisValue :type Float%20%28single-precision%29))
  (Pawn|Input|AddMovementInput (Pawn|GetControlledPawn) (Math|Vector|MakeVector (stale Input|AxisEvents|InputAxisMoveForward AxisValue) AxisValue 0.0) 1.0 false))

(event Input|AxisEvents|InputAxisMoveForward
  (params (AxisValue :type Float%20%28single-precision%29))
  (Pawn|Input|AddMovementInput (Pawn|GetControlledPawn) (Math|Vector|MakeVector AxisValue (stale Input|AxisEvents|InputAxisMoveRight AxisValue) 0.0) 1.0 false))

(fn ConstructionScript)